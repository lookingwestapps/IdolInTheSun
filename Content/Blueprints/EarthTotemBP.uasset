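; EarthTotemBP is an earth totem actor that respawns at its start location when it falls below world height zero.
; BeginPlay assigns a green ribbon effect and an earth explosion hit effect to its variables.
; Tick watches the Box component's height, then plays a splash sound, emits a spark above the start point, spawns a fresh copy there and destroys itself.
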(event `self.ReceiveBeginPlay`
  (set `self.RibbonEffect` "/Game/Particles/P_Ribbon_02GREEN.P_Ribbon_02GREEN")
  (set `self.ParticleEffectOnHit` "/Game/ParicleSystems/P_Earth_explosion.P_Earth_explosion"))

(event `self.ReceiveActorBeginOverlap`
  (params (OtherActor :type "Actor Object Reference")))

(event `self.ReceiveTick`
  (params (DeltaSeconds :type "Float (single-precision)"))
  (bind _startlocation (`self.StartLocation`))
  (bind _returnvalue (`SceneComponent.K2_GetComponentLocation` (`self.Box`)))
  (if (< (.z _returnvalue) 0.0)
    (`GameplayStatics.PlaySoundAtLocation` "/Game/Sounds/Boss_Miss_Splash_Final.Boss_Miss_Splash_Final" _returnvalue)
    (`GameplayStatics.SpawnEmitterAtLocation` "/Game/Particles/AppearSpark.AppearSpark" (+ _startlocation (0.0 0.0 25.0)))
    (`|SpawnActorFromClass` "EarthTotemBP_C" (`KismetMathLibrary.MakeTransform` _startlocation) "AdjustIfPossibleButAlwaysSpawn" "OverrideRootScale")
    (`self.K2_DestroyActor`)))

(fn `UserConstructionScript`
  (`parent.UserConstructionScript`))