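; Catapult actor that launches a loaded totem projectile and plays its firing animations and sounds.
; RunCatapultAnimation plays fire animations on the cog, launcher and wheels when a totem is loaded.
; FireCatapult enables physics on the totem, applies a velocity-change impulse with attached flight sound and ribbon effect, then clears the reference.
; ResetCatapult only plays a sound, and BeginPlay plays the launcher animation once to work around a visibility bug.
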(event `self.ReceiveBeginPlay`
  ;[1 1 1] Had to run this animation once at start to fix bug with launcher not showing
  (`SkeletalMeshComponent.PlayAnimation` (`self.catapult_launcher`) "/Game/Catapult/SM_Catapult_launcher_FIRE.SM_Catapult_launcher_FIRE" false))

(event `self.ReceiveActorBeginOverlap`
  (params (OtherActor :type "Actor Object Reference")))

(event `self.ReceiveTick`
  (params (DeltaSeconds :type "Float (single-precision)")))

(fn `FireCatapult`
  (bind _projectiletotem (`self.ProjectileTotem`))
  (bind _box (`/Game/Blueprints/Totem_BaseClass_BP.Box` _projectiletotem))
  (if (`KismetSystemLibrary.IsValid` _projectiletotem)
    (`GameplayStatics.PlaySoundAtLocation` "/Game/Sounds/Catapult_Launch_Final.Catapult_Launch_Final" (`SceneComponent.K2_GetComponentLocation` (`self.DefaultSceneRoot`)))
    (`GameplayStatics.SpawnSoundAttached` "/Game/Sounds/Totem_Flight_Final.Totem_Flight_Final" _box)
    (`GameplayStatics.SpawnEmitterAttached` (`/Game/Blueprints/Totem_BaseClass_BP.RibbonEffect` _projectiletotem) _box)
    (`PrimitiveComponent.SetSimulatePhysics` _box true)
    (`PrimitiveComponent.AddImpulse` _box (`self.Fire Impulse`) "None" true)
    (set `self.ProjectileTotem` null)))

(fn `ResetCatapult`
  (`GameplayStatics.PlaySoundAtLocation` "/Game/Sounds/Catapult_Reset_Final.Catapult_Reset_Final" (`SceneComponent.K2_GetComponentLocation` (`self.DefaultSceneRoot`))))

(fn `RunCatapultAnimation`
  (if (`KismetSystemLibrary.IsValid` (`self.ProjectileTotem`))
    (`SkeletalMeshComponent.PlayAnimation` (`self.catapult_cog`) "/Game/Catapult/SM_Catapult_cog_FIRE.SM_Catapult_cog_FIRE" false)
    (`SkeletalMeshComponent.PlayAnimation` (`self.catapult_launcher`) "/Game/Catapult/SM_Catapult_launcher_FIRE.SM_Catapult_launcher_FIRE" false)
    (`SkeletalMeshComponent.PlayAnimation` (`self.catapult_wheels`) "/Game/Catapult/SM_Catapult_wheel_FIRE.SM_Catapult_wheel_FIRE" false)))

(fn `UserConstructionScript`)