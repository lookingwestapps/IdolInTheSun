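; FireTotemBP is a fire totem actor that respawns at its start location after falling below world height zero.
; BeginPlay sets a red ribbon effect and a fire explosion hit effect for use outside this graph.
; Tick watches the Box component's height, then plays a splash sound, spawns a fresh copy at StartLocation and destroys itself.
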(event `self.ReceiveBeginPlay`
  (set `self.RibbonEffect` "/Game/Particles/P_Ribbon_02RED.P_Ribbon_02RED")
  (set `self.ParticleEffectOnHit` "/Game/ParicleSystems/P_fire_explosion.P_fire_explosion"))

(event `self.ReceiveActorBeginOverlap`
  (params (OtherActor :type "Actor Object Reference")))

(event `self.ReceiveTick`
  (params (DeltaSeconds :type "Float (single-precision)"))
  (bind _returnvalue (`SceneComponent.K2_GetComponentLocation` (`self.Box`)))
  (if (< (.z _returnvalue) 0.0)
    (`GameplayStatics.PlaySoundAtLocation` "/Game/Sounds/Boss_Miss_Splash_Final.Boss_Miss_Splash_Final" _returnvalue)
    (`|SpawnActorFromClass` "FireTotemBP_C" (`KismetMathLibrary.MakeTransform` (`self.StartLocation`)) "AdjustIfPossibleButAlwaysSpawn" "OverrideRootScale")
    (`self.K2_DestroyActor`)))

(fn `UserConstructionScript`
  (`parent.UserConstructionScript`))