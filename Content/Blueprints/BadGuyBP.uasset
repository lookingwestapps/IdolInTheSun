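; Sun god boss that loops along a spline, opening and closing its mouth until totem hits kill it.
; Tick advances spline distance, then reruns the BeginPlay chain to set position, derive the mouth morph target from spline-point segments, and play open/close sounds.
; Totem hits play random sounds and effects, briefly halt movement and destroy the totem; the third makes the boss fall away spinning.
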(event `self.ReceiveBeginPlay`
  (bind _splinedistance (`self.SplineDistance`))
  (bind _returnvalue (`SceneComponent.K2_GetComponentLocation` (`self.DefaultSceneRoot`)))
  (bind _spline (`/Game/Blueprints/SplineBP.Spline` (`self.Spline_BP`)))
  (bind _returnvalue_2 (`SplineComponent.GetDistanceAlongSplineAtSplinePoint` _spline 5))
  (bind _returnvalue_3 (`SplineComponent.GetDistanceAlongSplineAtSplinePoint` _spline 3))
  (bind _returnvalue_4 (`SplineComponent.GetDistanceAlongSplineAtSplinePoint` _spline 1))
  (bind _returnvalue_5 (`SplineComponent.GetDistanceAlongSplineAtSplinePoint` _spline 2))
  (bind _returnvalue_6 (`SplineComponent.GetDistanceAlongSplineAtSplinePoint` _spline 4))
  ;[1 1 1] Get/Set Location based on Current Position on Spline
  (`SceneComponent.K2_SetWorldLocation` (`self.DefaultSceneRoot`) (`SplineComponent.GetLocationAtDistanceAlongSpline` _spline _splinedistance "World") false false :!label _label)
  (if (> _splinedistance _returnvalue_4)
    (if (> _splinedistance _returnvalue_3)
      (if (> _splinedistance _returnvalue_6)
        ;[1 1 1] Set from 4-5
        (`SkeletalMeshComponent.SetMorphTarget` (`self.SkeletalMesh`) "GJ_SunGod3" (`KismetMathLibrary.FClamp` (/ (- _returnvalue_2 _splinedistance) (- _returnvalue_2 _returnvalue_6))) true)
        ;[1 1 1] Mouth Open/Close Sound Effects
        (if (`self.MouthOpen`) :!label _label_2
          (set `self.MouthOpen` false)
          (`GameplayStatics.PlaySoundAtLocation` "/Game/Sounds/mouth_close.mouth_close" _returnvalue))
        (else
          ;[1 1 1] Set from 3-4
          (`SkeletalMeshComponent.SetMorphTarget` (`self.SkeletalMesh`) "GJ_SunGod3" (`KismetMathLibrary.FClamp` (- 1.0 (/ (- _returnvalue_6 _splinedistance) (- _returnvalue_6 _returnvalue_3)))) true)
          (if (not (`self.MouthOpen`)) :!label _label_3
            (set `self.MouthOpen` true)
            (`GameplayStatics.PlaySoundAtLocation` "/Game/Sounds/mouth_open.mouth_open" _returnvalue))))
      (else
        ;[1 1 1] Set from 1-2
        (`SkeletalMeshComponent.SetMorphTarget` (`self.SkeletalMesh`) "GJ_SunGod3" (`KismetMathLibrary.FClamp` (/ (- _returnvalue_5 _splinedistance) (- _returnvalue_5 _returnvalue_4))) true)
        (goto _label_2)))
    (else
      ;[1 1 1] Set from 0-1
      (`SkeletalMeshComponent.SetMorphTarget` (`self.SkeletalMesh`) "GJ_SunGod3" (/ _splinedistance _returnvalue_4) true)
      (goto _label_3))))

(event `self.ReceiveActorBeginOverlap`
  (params (OtherActor :type "Actor Object Reference")))

(event `self.ReceiveTick`
  (params (DeltaSeconds :type "Float (single-precision)"))
  (bind _spline (`/Game/Blueprints/SplineBP.Spline` (`self.Spline_BP`)))
  ;[1 1 1] Move the Sun along the Spline
  (if (not (`self.Dead`))
    (set `self.SplineDistance` (+ (* DeltaSeconds (`self.Speed`)) (`self.SplineDistance`)))
    ;[1 1 1] Loop to start of spline when done
    (if (== (`SplineComponent.GetLocationAtSplinePoint` _spline (`SplineComponent.GetNumberOfSplinePoints` _spline) "World") (`SplineComponent.GetLocationAtDistanceAlongSpline` _spline (`self.SplineDistance`) "World"))
      (set `self.SplineDistance` 0.0)
      (goto _label)
      (else
        (goto _label)))))

(event `self.ReceiveHit`
  (params (MyComp :type "PrimitiveComponent Object Reference") (Other :type "Actor Object Reference") (OtherComp :type "PrimitiveComponent Object Reference") (bSelfMoved :type Boolean) (HitLocation :type "Vector Structure") (HitNormal :type "Vector Structure") (NormalImpulse :type "Vector Structure") (Hit :type "HitResult Structure (by ref)"))
  (bind _returnvalue (`self.K2_GetRootComponent`))
  (bind (_bblockinghit _binitialoverlap _time _location _impactpoint _normal _impactnormal _physmat _hitactor) (`GameplayStatics.BreakHitResult` Hit))
  (bind _hitcounter (`self.HitCounter`))
  (bind _returnvalue_2 (`SceneComponent.K2_GetComponentLocation` _returnvalue))
  ;[1 1 1] Totem has hit Sun Mouth
  (bind _newparam (`self.PickSound`))
  (`GameplayStatics.PlaySoundAtLocation` _newparam (`self.K2_GetActorLocation` _hitactor))
  (bind _astotem_base_class_bp (cast `/Game/Blueprints/Totem_BaseClass_BP` _hitactor))
  (`GameplayStatics.SpawnEmitterAtLocation` (`/Game/Blueprints/Totem_BaseClass_BP.ParticleEffectOnHit` _astotem_base_class_bp) _impactpoint)
  (set `self.Speed` 0.0)
  (`self.K2_DestroyActor` _hitactor)
  (set `self.HitCounter` (+ _hitcounter 1))
  (`KismetSystemLibrary.Delay` 0.5)
  (set `self.Speed` 5000.0)
  (if (>= _hitcounter 3)
    ;[1 1 1] SunGod Death
    (set `self.Dead` true) ; Stop Moving on Spline
    (`KismetSystemLibrary.Delay` 1.0)
    (`GameplayStatics.PlaySoundAtLocation` "/Game/Sounds/death_sound.death_sound" _returnvalue_2)
    (`KismetSystemLibrary.MoveComponentTo` _returnvalue (+ _returnvalue_2 (0.0 0.0 -70000.0)) (`KismetMathLibrary.MakeRotator` (`KismetMathLibrary.RandomFloatInRange` 0.0 200.0) (`KismetMathLibrary.RandomFloatInRange` 0.0 200.0) (`KismetMathLibrary.RandomFloatInRange` 0.0 200.0)) true true 6.0)))

(fn `PickSound`
  (returns (NewParam :type "SoundWave Object Reference"))
  (return (`KismetArrayLibrary.Array_Get` (`|MakeArray` (`self.Sound1`) (`self.Sound2`) (`self.Sound3`) (`self.Sound4`) (`self.Sound5`) (`self.Sound6`) (`self.Sound7`) (`self.Sound8`)) (`KismetMathLibrary.RandomInteger` 7))))

(fn `UserConstructionScript`)